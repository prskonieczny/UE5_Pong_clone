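; Pong controller Blueprint that moves both paddles and runs the match from main menu to end screen.
; BeginPlay shows the menu and spawns the ball, which W or S launches once starting is allowed.
; Tick fans out into handlers that poll keys for wall-limited paddle movement and count down the timer.
; Reaching max score or zero time destroys the ball and shows the end widget, while SpawnBall launches replacement balls.
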(event Custom|Tick2
  (params (Delta%20Seconds :type Float%20%28double-precision%29))
  (bind _returnvalue (Game|GetPlayerController 0))
  (bind _players_speed_down (Variables|Default|Getplayers_speed_down))
  ;[1 1 1] Ruch lewego gracza w dół
  (if (Game|Player|IsInputKeyDown _returnvalue (stale Input|KeyboardEvents|S Key))
    (if (< (.x (Transformation|GetWorldLocation (Variables|Default|GetPlayer_L))) (Variables|Default|GetWall2Location))
      (Transformation|AddLocalOffset (Variables|Default|GetPlayer_L) (Math|Vector|MakeVector (* Delta%20Seconds _players_speed_down) 0.0 0.0) false false)))
  ;[1 1 1] Ruch prawego gracza w dół
  (if (Game|Player|IsInputKeyDown _returnvalue (stale Input|KeyboardEvents|Down Key))
    (if (< (.x (Transformation|GetWorldLocation (Variables|Default|GetPlayer_R))) (Variables|Default|GetWall2Location))
      (Transformation|AddLocalOffset (Variables|Default|GetPlayer_R) (Math|Vector|MakeVector (* Delta%20Seconds _players_speed_down) 0.0 0.0) false false))))

(event Custom|Tick%203
  (params (Delta%20Seconds :type Float%20%28double-precision%29))
  (bind _returnvalue (Game|GetPlayerController 0))
  (bind _players_speed_up (Variables|Default|Getplayers_speed_up))
  ;[1 1 1] Warunek końca - czas
  (if (Variables|Default|GetCurrentlyPlaying)
    (bind _output_get (Variables|Default|SetcurrTime (- (Variables|Default|GetcurrTime) Delta%20Seconds)))
    ;[1 1 1] Warunek końca - wynik
    (if (<= (Variables|Default|GetMaxScore) (Variables|Default|GetScoreLeft))
      ;[1 1 1] Zakonczenie
      (Variables|Default|SetCurrentlyPlaying false :!label _label)
      ;[1 1 1] End Screen
      (Variables|Default|SetcurrTime 0.0)
      (Viewport|RemoveAllWidgets)
      (bind _returnvalue_2 (UserInterface|CreateWidget "/Game/Pong_Clone/Blueprints/WBP_End.WBP_End_C"))
      (UserInterface|Viewport|AddtoViewport _returnvalue_2 0)
      (bind _returnvalue_3 (Actor|GetActorOfClass "/Game/Pong_Clone/Blueprints/BP_Ball.BP_Ball_C"))
      (Actor|DestroyActor _returnvalue_3)
      (elif (<= (Variables|Default|GetMaxScore) (Variables|Default|GetScoreRight))
        (goto _label)
        (elif (< _output_get 0.0)
          (goto _label)
          (else
            ;[1 1 1] Ruch lewego gracza w górę
            (if (Game|Player|IsInputKeyDown _returnvalue (stale Input|KeyboardEvents|W Key))
              (if (< (Variables|Default|GetWall1Location) (.x (Transformation|GetWorldLocation (Variables|Default|GetPlayer_L))))
                (Transformation|AddLocalOffset (Variables|Default|GetPlayer_L) (Math|Vector|MakeVector (* (stale Custom|Tick1 Delta%20Seconds) _players_speed_up) 0.0 0.0) false false)))
            ;[1 1 1] Ruch prawego gracza w górę
            (if (Game|Player|IsInputKeyDown _returnvalue (stale Input|KeyboardEvents|Up Key))
              (if (< (Variables|Default|GetWall1Location) (.x (Transformation|GetWorldLocation (Variables|Default|GetPlayer_R))))
                (Transformation|AddLocalOffset (Variables|Default|GetPlayer_R) (Math|Vector|MakeVector (* (stale Custom|Tick1 Delta%20Seconds) _players_speed_up) 0.0 0.0) false false)))))))))

(event Custom|Tick1
  (params (Delta%20Seconds :type Float%20%28double-precision%29))
  (bind _returnvalue (Game|GetPlayerController 0))
  (bind _players_speed_up (Variables|Default|Getplayers_speed_up))
  ;[1 1 1] Ruch lewego gracza w górę
  (if (Game|Player|IsInputKeyDown _returnvalue (stale Input|KeyboardEvents|W Key))
    (if (< (Variables|Default|GetWall1Location) (.x (Transformation|GetWorldLocation (Variables|Default|GetPlayer_L))))
      (Transformation|AddLocalOffset (Variables|Default|GetPlayer_L) (Math|Vector|MakeVector (* Delta%20Seconds _players_speed_up) 0.0 0.0) false false)))
  ;[1 1 1] Ruch prawego gracza w górę
  (if (Game|Player|IsInputKeyDown _returnvalue (stale Input|KeyboardEvents|Up Key))
    (if (< (Variables|Default|GetWall1Location) (.x (Transformation|GetWorldLocation (Variables|Default|GetPlayer_R))))
      (Transformation|AddLocalOffset (Variables|Default|GetPlayer_R) (Math|Vector|MakeVector (* Delta%20Seconds _players_speed_up) 0.0 0.0) false false))))

(event Custom|SpawnBall
  ;[1 1 1] Spawn piłki po uderzeniu w sciane i nadanie jej predkosci
  (bind _returnvalue (Game|SpawnActorfromClass "/Game/Pong_Clone/Blueprints/BP_Ball.BP_Ball_C" (Math|Transform|MakeTransform "0,1000.000000,300.000000" "0, 0, 0" "1.000000,1.000000,1.000000") "Undefined" 0 0))
  (Default|RandomDirection _returnvalue))

(event EventBeginPlay
  ;[1 1 1] Wyswietlenie main menu
  (bind _returnvalue (UserInterface|CreateWidget "/Game/Pong_Clone/Blueprints/WBP_MainMenu.WBP_MainMenu_C"))
  (UserInterface|Viewport|AddtoViewport _returnvalue 0)
  (bind _returnvalue_2 (Game|SpawnActorfromClass "/Game/Pong_Clone/Blueprints/BP_Ball.BP_Ball_C" (Math|Transform|MakeTransform "0.000000,1000.000000,300.000000" "0, 0, 0" "1.000000,1.000000,1.000000") "Undefined" 0 0)))

(event EventTick
  (params (DeltaSeconds :type Float%20%28single-precision%29))
  ;[1 1 1] Powielenie Tick Events
  (CallFunction|Tick1 DeltaSeconds)
  (CallFunction|Tick2 DeltaSeconds)
  (CallFunction|Tick3 DeltaSeconds))

(event Input|KeyboardEvents|S
  (params (Key :type Key%20Structure :default "None"))
  ;[1 1 1] Ruch lewego gracza w dół
  (:Pressed
    ;[1 1 1] Czy mozna zaczac gre?
    (if (Variables|Default|GetcanStart?)
      (if (not (Variables|Default|GetCurrentlyPlaying))
        (Variables|Default|SetcanStart? false)
        (Variables|Default|SetCurrentlyPlaying true)
        (Default|RandomDirection (stale EventBeginPlay _returnvalue_2))))))

(event Input|KeyboardEvents|W
  (params (Key :type Key%20Structure :default "None"))
  ;[1 1 1] Ruch lewego gracza w górę
  (:Pressed
    ;[1 1 1] Czy mozna zaczac gre?
    (if (Variables|Default|GetcanStart?)
      (if (not (Variables|Default|GetCurrentlyPlaying))
        (Variables|Default|SetcanStart? false)
        (Variables|Default|SetCurrentlyPlaying true)
        (Default|RandomDirection (stale EventBeginPlay _returnvalue_2))))))

(event Input|KeyboardEvents|Up
  (params (Key :type Key%20Structure :default "None"))
  ;[1 1 1] Ruch prawego gracza w górę
  (:Pressed
    (if (Game|Player|IsInputKeyDown (Game|GetPlayerController 0) Key)
      (if (< (Variables|Default|GetWall1Location) (.x (Transformation|GetWorldLocation (Variables|Default|GetPlayer_R))))
        (Transformation|AddLocalOffset (Variables|Default|GetPlayer_R) (Math|Vector|MakeVector (* (stale Custom|Tick1 Delta%20Seconds) (Variables|Default|Getplayers_speed_up)) 0.0 0.0) false false)))))

(event Input|KeyboardEvents|Down
  (params (Key :type Key%20Structure :default "None"))
  ;[1 1 1] Ruch prawego gracza w dół
  (:Pressed
    (if (Game|Player|IsInputKeyDown (Game|GetPlayerController 0) Key)
      (if (< (.x (Transformation|GetWorldLocation (Variables|Default|GetPlayer_R))) (Variables|Default|GetWall2Location))
        (Transformation|AddLocalOffset (Variables|Default|GetPlayer_R) (Math|Vector|MakeVector (* (stale Custom|Tick2 Delta%20Seconds) (Variables|Default|Getplayers_speed_down)) 0.0 0.0) false false)))))

(fn ConstructionScript)